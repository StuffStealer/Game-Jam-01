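; AI controller for guard enemies that runs the guard behavior tree on BeginPlay.
; When its AI perception updates, it checks each updated actor for the player class.
; For the player, it displays the eyes message on them and sets the "Attacking?" blackboard key to true.
; The handler never checks whether the stimulus was sensed or lost, and nothing here clears the key.
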(event OnPerceptionUpdated(AIPerception)
  (params (UpdatedActors :type Array%20of%20Actor%20Object%20References))
  (for _array_element UpdatedActors
    (if (== (Utilities|GetClass _array_element) "/Game/Blueprints/Player/BP_Player.BP_Player_C")
      (Class|BPIDetection|DisplayEyes(Message) _array_element)
      (AI|Components|Blackboard|SetValueasBool (AI|GetBlackboard self) (Utilities|Name|MakeLiteralName "Attacking?") true))))

(event EventBeginPlay
  (AI|RunBehaviorTree self "/Game/Blueprints/IA/BP_BT_Enemy_Guard.BP_BT_Enemy_Guard"))

(event EventTick
  (params (DeltaSeconds :type Float%20%28single-precision%29)))

(fn ConstructionScript)