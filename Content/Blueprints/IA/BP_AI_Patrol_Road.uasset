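; BP_AI_Patrol_Road is a spline-based patrol route for AI, supplying one patrol point at a time.
; Increment_Patrol_Road steps PatrolIndex by Direction, flipping Direction at the last and first spline points so the route runs back and forth instead of looping.
; GetSplineAsWorldPosiiton returns the world location of the current PatrolRoad point.
; It has no active BeginPlay or Tick logic, so advancing relies on external calls.
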(event Custom|Increment_Patrol_Road
  (bind _output_get (Variables|Default|SetPatrol_Index (+ (Variables|Default|GetPatrol_Index) (Variables|Default|GetDirection))))
  (if (== _output_get (- (Spline|GetNumberOfSplinePoints (Variables|Default|GetPatrol_Road)) 1))
    (Variables|Default|SetDirection -1)
    (elif (== (Variables|Default|GetPatrol_Index) 0)
      (Variables|Default|SetDirection 1))))

(event EventBeginPlay)

(event Collision|EventActorBeginOverlap
  (params (OtherActor :type Actor%20Object%20Reference)))

(event EventTick
  (params (DeltaSeconds :type Float%20%28single-precision%29)))

(fn ConstructionScript)

(fn GetSplineasWorldPosiiton
  (return (Spline|GetLocationatSplinePoint (Variables|Default|GetPatrol_Road) (Variables|Default|GetPatrol_Index) "World")))