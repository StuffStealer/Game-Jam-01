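; Master enemy Blueprint for NPCs that the player hunts: any damage destroys it and reports victory or failure by matching its thumbnail to the player's wanted target.
; Each tick, sphere traces for the player reveal a trail effect at long range and drive cross-particle visibility and spawn rate in closer distance bands.
; It also provides events to show or collapse its word widgets and exposes its patrol road.
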(event Custom|Hidden_Widget_Word
  (if (Utilities|Array|IsNotEmpty (Variables|Default|GetWidget_Array))
    (for _array_element (Variables|Default|GetWidget_Array)
      (Variables|/Script/UMG.Widget|SetVisibility _array_element "Collapsed"))))

(event Custom|Display_Widget_Word
  (if (Utilities|Array|IsNotEmpty (Variables|Default|GetWidget_Array))
    (for _array_element (Variables|Default|GetWidget_Array)
      (Variables|/Script/UMG.Widget|SetVisibility _array_element "Visible"))))

(event Collision|EventActorBeginOverlap
  (params (OtherActor :type Actor%20Object%20Reference)))

(event EventTick
  (params (DeltaSeconds :type Float%20%28single-precision%29))
  (bind _mesh (Variables|Character|GetMesh))
  (bind _fx_cross_particles (Variables|Default|GetFX_Cross_Particles))
  (bind _fx_cross_particles_2 (Variables|Default|GetFX_Cross_Particles))
  (bind _fx_cross_particles_3 (Variables|Default|GetFX_Cross_Particles))
  (bind _fx_cross_particles_4 (Variables|Default|GetFX_Cross_Particles))
  (bind _mesh_2 (Variables|Character|GetMesh))
  (bind _returnvalue (Transformation|GetWorldLocation _mesh_2))
  (bind _returnvalue_2 (Transformation|GetWorldLocation _mesh))
  (Utilities|FlowControl|Sequence
    (:then_0
      (bind (_outhits _returnvalue_3) (Collision|MultiSphereTraceForObjects _returnvalue_2 _returnvalue_2 7.5e+03 (Utilities|Array|MakeArray "ObjectTypeQuery3") false 0 "None" true "(R=0.000000,G=0.051031,B=1.000000,A=1.000000)" "(R=0.000000,G=1.000000,B=0.826785,A=1.000000)"))
      (if _returnvalue_3
        (for _array_element _outhits
          (if (== (Utilities|GetClass (.HitActor (Collision|BreakHitResult _array_element))) "/Game/Blueprints/Player/BP_Player.BP_Player_C")
            (Development|SetHiddeninGame (Variables|Default|GetNG_Trail) false false)))
        (else
          (Development|SetHiddeninGame (Variables|Default|GetNG_Trail) true false))))
    (:then_1
      (bind (_outhits_2 _returnvalue_4) (Collision|MultiSphereTraceForObjects _returnvalue _returnvalue 4e+03 (Utilities|Array|MakeArray "ObjectTypeQuery3") false 0 "None" true "(R=1.000000,G=0.000000,B=0.592295,A=1.000000)" "(R=1.000000,G=0.000000,B=0.028412,A=1.000000)"))
      (if _returnvalue_4
        (for _array_element_2 _outhits_2
          (if (== (Utilities|GetClass (.HitActor (Collision|BreakHitResult _array_element_2))) "/Game/Blueprints/Player/BP_Player.BP_Player_C")
            (Utilities|FlowControl|Sequence
              (:then_0
                (if (>= (Math|Vector|Distance(Vector) (Transformation|GetActorLocation (.HitActor (Collision|BreakHitResult _array_element_2))) (Transformation|GetActorLocation)) 3e+03)
                  (Development|SetHiddeninGame _fx_cross_particles true false)
                  (Niagara|SetNiagaraVariable(Float) _fx_cross_particles "SpawnRate" 0.0)))
              (:then_1
                (if (<= (Math|Vector|Distance(Vector) (Transformation|GetActorLocation (.HitActor (Collision|BreakHitResult _array_element_2))) (Transformation|GetActorLocation)) 3e+03)
                  (if (<= (Math|Vector|Distance(Vector) (Transformation|GetActorLocation (.HitActor (Collision|BreakHitResult _array_element_2))) (Transformation|GetActorLocation)) 1.5e+03)
                    (Development|SetHiddeninGame _fx_cross_particles_2 false false)
                    (Niagara|SetNiagaraVariable(Float) _fx_cross_particles_2 "SpawnRate" 1e+01)
                    (else
                      (Development|SetHiddeninGame _fx_cross_particles_4 false false)
                      (Niagara|SetNiagaraVariable(Float) _fx_cross_particles_4 "SpawnRate" 1.0))))))))
        (else
          (Development|SetHiddeninGame _fx_cross_particles_3 true false)
          (Niagara|SetNiagaraVariable(Float) _fx_cross_particles_3 "SpawnRate" 0.0))))))

(event Game|Damage|EventAnyDamage
  (params (Damage :type Float%20%28single-precision%29) (DamageType :type Damage%20Type%20Object%20Reference) (InstigatedBy :type Controller%20Object%20Reference) (DamageCauser :type Actor%20Object%20Reference))
  (Actor|DestroyActor)
  (bind _asbp_player (Utilities|Casting|CastToBP_Player (Game|GetPlayerCharacter 0)))
  (if (== (Variables|/Game/Blueprints/Player/BP_Player.BP_Player_C|GetRef_Wanted_Game _asbp_player) (Utilities|Struct|BreakStruct_PNJ (Variables|Setup|GetStruct_PNJ)))
    (Default|VictorySetup _asbp_player true)
    (else
      (Default|VictorySetup _asbp_player false))))

(fn ConstructionScript)

(fn GetPatrolRoad
  (return (Variables|Default|GetPatrol_Road)))